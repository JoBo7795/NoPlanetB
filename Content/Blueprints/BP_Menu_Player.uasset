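; Menu player that forwards mouse clicks and typing to UMG widgets through its WidgetInteractionMouse component.
; Hard-coded key events send characters for a German keyboard layout, choosing shifted variants from one ShiftClicked flag that both Shifts set and CapsLock flips.
; Numpad digits reuse the unshifted digit sends, while left mouse, Backspace and Delete are forwarded as pointer or key presses.
; The InputCharacter function is an empty, unused stub.
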(event EventBeginPlay)

(event Collision|EventActorBeginOverlap
  (params (OtherActor :type Actor%20Object%20Reference)))

(event EventTick
  (params (DeltaSeconds :type Float%20%28single-precision%29)))

(event Input|MouseEvents|LeftMouseButton
  (params (Key :type Key%20Structure :default "None"))
  (bind _widgetinteractionmouse (Variables|Default|GetWidgetInteractionMouse))
  ;[1 1 1] Mouse
  (:Pressed
    (Class|WidgetInteractionComponent|PressPointerKey _widgetinteractionmouse "LeftMouseButton"))
  (:Released
    (Class|WidgetInteractionComponent|ReleasePointerKey _widgetinteractionmouse "LeftMouseButton")))

(event Input|KeyboardEvents|NumPadNine
  (params (Key :type Key%20Structure :default "None"))
  ;[1 1 1] 0-9, !-=
  (:Pressed
    (Class|WidgetInteractionComponent|SendKeyChar (Variables|Default|GetWidgetInteractionMouse) "9" false)))

(event Input|KeyboardEvents|7
  (params (Key :type Key%20Structure :default "None"))
  (bind _widgetinteractionmouse (Variables|Default|GetWidgetInteractionMouse))
  ;[1 1 1] 0-9, !-=
  (:Pressed
    (if (Variables|Default|GetshiftClicked)
      (Class|WidgetInteractionComponent|SendKeyChar _widgetinteractionmouse "/" false)
      (else
        (Class|WidgetInteractionComponent|SendKeyChar _widgetinteractionmouse "7" false)))))

(event Input|KeyboardEvents|8
  (params (Key :type Key%20Structure :default "None"))
  (bind _widgetinteractionmouse (Variables|Default|GetWidgetInteractionMouse))
  ;[1 1 1] 0-9, !-=
  (:Pressed
    (if (Variables|Default|GetshiftClicked)
      (Class|WidgetInteractionComponent|SendKeyChar _widgetinteractionmouse "(" false)
      (else
        (Class|WidgetInteractionComponent|SendKeyChar _widgetinteractionmouse "8" false)))))

(event Input|KeyboardEvents|9
  (params (Key :type Key%20Structure :default "None"))
  (bind _widgetinteractionmouse (Variables|Default|GetWidgetInteractionMouse))
  ;[1 1 1] 0-9, !-=
  (:Pressed
    (if (Variables|Default|GetshiftClicked)
      (Class|WidgetInteractionComponent|SendKeyChar _widgetinteractionmouse ")" false)
      (else
        (Class|WidgetInteractionComponent|SendKeyChar _widgetinteractionmouse "9" false)))))

(event Input|KeyboardEvents|A
  (params (Key :type Key%20Structure :default "None"))
  (bind _widgetinteractionmouse (Variables|Default|GetWidgetInteractionMouse))
  ;[1 1 1] a-z, A-Z und die ganzen anderen Tasten auch, außer Tab und so
  (:Pressed
    (if (Variables|Default|GetshiftClicked)
      (Class|WidgetInteractionComponent|SendKeyChar _widgetinteractionmouse "A" false)
      (else
        (Class|WidgetInteractionComponent|SendKeyChar _widgetinteractionmouse "a" false)))))

(event Input|KeyboardEvents|B
  (params (Key :type Key%20Structure :default "None"))
  (bind _widgetinteractionmouse (Variables|Default|GetWidgetInteractionMouse))
  ;[1 1 1] a-z, A-Z und die ganzen anderen Tasten auch, außer Tab und so
  (:Pressed
    (if (Variables|Default|GetshiftClicked)
      (Class|WidgetInteractionComponent|SendKeyChar _widgetinteractionmouse "B" false)
      (else
        (Class|WidgetInteractionComponent|SendKeyChar _widgetinteractionmouse "b" false)))))

(event Input|KeyboardEvents|C
  (params (Key :type Key%20Structure :default "None"))
  (bind _widgetinteractionmouse (Variables|Default|GetWidgetInteractionMouse))
  ;[1 1 1] a-z, A-Z und die ganzen anderen Tasten auch, außer Tab und so
  (:Pressed
    (if (Variables|Default|GetshiftClicked)
      (Class|WidgetInteractionComponent|SendKeyChar _widgetinteractionmouse "C" false)
      (else
        (Class|WidgetInteractionComponent|SendKeyChar _widgetinteractionmouse "c" false)))))

(event Input|KeyboardEvents|D
  (params (Key :type Key%20Structure :default "None"))
  (bind _widgetinteractionmouse (Variables|Default|GetWidgetInteractionMouse))
  ;[1 1 1] a-z, A-Z und die ganzen anderen Tasten auch, außer Tab und so
  (:Pressed
    (if (Variables|Default|GetshiftClicked)
      (Class|WidgetInteractionComponent|SendKeyChar _widgetinteractionmouse "D" false)
      (else
        (Class|WidgetInteractionComponent|SendKeyChar _widgetinteractionmouse "d" false)))))

(event Input|KeyboardEvents|E
  (params (Key :type Key%20Structure :default "None"))
  (bind _widgetinteractionmouse (Variables|Default|GetWidgetInteractionMouse))
  ;[1 1 1] a-z, A-Z und die ganzen anderen Tasten auch, außer Tab und so
  (:Pressed
    (if (Variables|Default|GetshiftClicked)
      (Class|WidgetInteractionComponent|SendKeyChar _widgetinteractionmouse "E" false)
      (else
        (Class|WidgetInteractionComponent|SendKeyChar _widgetinteractionmouse "e" false)))))

(event Input|KeyboardEvents|F
  (params (Key :type Key%20Structure :default "None"))
  (bind _widgetinteractionmouse (Variables|Default|GetWidgetInteractionMouse))
  ;[1 1 1] a-z, A-Z und die ganzen anderen Tasten auch, außer Tab und so
  (:Pressed
    (if (Variables|Default|GetshiftClicked)
      (Class|WidgetInteractionComponent|SendKeyChar _widgetinteractionmouse "F" false)
      (else
        (Class|WidgetInteractionComponent|SendKeyChar _widgetinteractionmouse "f" false)))))

(event Input|KeyboardEvents|G
  (params (Key :type Key%20Structure :default "None"))
  (bind _widgetinteractionmouse (Variables|Default|GetWidgetInteractionMouse))
  ;[1 1 1] a-z, A-Z und die ganzen anderen Tasten auch, außer Tab und so
  (:Pressed
    (if (Variables|Default|GetshiftClicked)
      (Class|WidgetInteractionComponent|SendKeyChar _widgetinteractionmouse "G" false)
      (else
        (Class|WidgetInteractionComponent|SendKeyChar _widgetinteractionmouse "g" false)))))

(event Input|KeyboardEvents|1
  (params (Key :type Key%20Structure :default "None"))
  (bind _widgetinteractionmouse (Variables|Default|GetWidgetInteractionMouse))
  ;[1 1 1] 0-9, !-=
  (:Pressed
    (if (Variables|Default|GetshiftClicked)
      (Class|WidgetInteractionComponent|SendKeyChar _widgetinteractionmouse "!" false)
      (else
        (Class|WidgetInteractionComponent|SendKeyChar _widgetinteractionmouse "1" false)))))

(event Input|KeyboardEvents|H
  (params (Key :type Key%20Structure :default "None"))
  (bind _widgetinteractionmouse (Variables|Default|GetWidgetInteractionMouse))
  ;[1 1 1] a-z, A-Z und die ganzen anderen Tasten auch, außer Tab und so
  (:Pressed
    (if (Variables|Default|GetshiftClicked)
      (Class|WidgetInteractionComponent|SendKeyChar _widgetinteractionmouse "H" false)
      (else
        (Class|WidgetInteractionComponent|SendKeyChar _widgetinteractionmouse "h" false)))))

(event Input|KeyboardEvents|I
  (params (Key :type Key%20Structure :default "None"))
  (bind _widgetinteractionmouse (Variables|Default|GetWidgetInteractionMouse))
  ;[1 1 1] a-z, A-Z und die ganzen anderen Tasten auch, außer Tab und so
  (:Pressed
    (if (Variables|Default|GetshiftClicked)
      (Class|WidgetInteractionComponent|SendKeyChar _widgetinteractionmouse "I" false)
      (else
        (Class|WidgetInteractionComponent|SendKeyChar _widgetinteractionmouse "i" false)))))

(event Input|KeyboardEvents|J
  (params (Key :type Key%20Structure :default "None"))
  (bind _widgetinteractionmouse (Variables|Default|GetWidgetInteractionMouse))
  ;[1 1 1] a-z, A-Z und die ganzen anderen Tasten auch, außer Tab und so
  (:Pressed
    (if (Variables|Default|GetshiftClicked)
      (Class|WidgetInteractionComponent|SendKeyChar _widgetinteractionmouse "J" false)
      (else
        (Class|WidgetInteractionComponent|SendKeyChar _widgetinteractionmouse "j" false)))))

(event Input|KeyboardEvents|#
  (params (Key :type Key%20Structure :default "None"))
  (bind _widgetinteractionmouse (Variables|Default|GetWidgetInteractionMouse))
  ;[1 1 1] a-z, A-Z und die ganzen anderen Tasten auch, außer Tab und so
  (:Pressed
    (if (Variables|Default|GetshiftClicked)
      (Class|WidgetInteractionComponent|SendKeyChar _widgetinteractionmouse "'" false)
      (else
        (Class|WidgetInteractionComponent|SendKeyChar _widgetinteractionmouse "#" false)))))

(event Input|KeyboardEvents|K
  (params (Key :type Key%20Structure :default "None"))
  (bind _widgetinteractionmouse (Variables|Default|GetWidgetInteractionMouse))
  ;[1 1 1] a-z, A-Z und die ganzen anderen Tasten auch, außer Tab und so
  (:Pressed
    (if (Variables|Default|GetshiftClicked)
      (Class|WidgetInteractionComponent|SendKeyChar _widgetinteractionmouse "K" false)
      (else
        (Class|WidgetInteractionComponent|SendKeyChar _widgetinteractionmouse "k" false)))))

(event Input|KeyboardEvents|L
  (params (Key :type Key%20Structure :default "None"))
  (bind _widgetinteractionmouse (Variables|Default|GetWidgetInteractionMouse))
  ;[1 1 1] a-z, A-Z und die ganzen anderen Tasten auch, außer Tab und so
  (:Pressed
    (if (Variables|Default|GetshiftClicked)
      (Class|WidgetInteractionComponent|SendKeyChar _widgetinteractionmouse "L" false)
      (else
        (Class|WidgetInteractionComponent|SendKeyChar _widgetinteractionmouse "l" false)))))

(event Input|KeyboardEvents|M
  (params (Key :type Key%20Structure :default "None"))
  (bind _widgetinteractionmouse (Variables|Default|GetWidgetInteractionMouse))
  ;[1 1 1] a-z, A-Z und die ganzen anderen Tasten auch, außer Tab und so
  (:Pressed
    (if (Variables|Default|GetshiftClicked)
      (Class|WidgetInteractionComponent|SendKeyChar _widgetinteractionmouse "M" false)
      (else
        (Class|WidgetInteractionComponent|SendKeyChar _widgetinteractionmouse "m" false)))))

(event Input|KeyboardEvents|N
  (params (Key :type Key%20Structure :default "None"))
  (bind _widgetinteractionmouse (Variables|Default|GetWidgetInteractionMouse))
  ;[1 1 1] a-z, A-Z und die ganzen anderen Tasten auch, außer Tab und so
  (:Pressed
    (if (Variables|Default|GetshiftClicked)
      (Class|WidgetInteractionComponent|SendKeyChar _widgetinteractionmouse "N" false)
      (else
        (Class|WidgetInteractionComponent|SendKeyChar _widgetinteractionmouse "n" false)))))

(event Input|KeyboardEvents|O
  (params (Key :type Key%20Structure :default "None"))
  (bind _widgetinteractionmouse (Variables|Default|GetWidgetInteractionMouse))
  ;[1 1 1] a-z, A-Z und die ganzen anderen Tasten auch, außer Tab und so
  (:Pressed
    (if (Variables|Default|GetshiftClicked)
      (Class|WidgetInteractionComponent|SendKeyChar _widgetinteractionmouse "O" false)
      (else
        (Class|WidgetInteractionComponent|SendKeyChar _widgetinteractionmouse "o" false)))))

(event Input|KeyboardEvents|P
  (params (Key :type Key%20Structure :default "None"))
  (bind _widgetinteractionmouse (Variables|Default|GetWidgetInteractionMouse))
  ;[1 1 1] a-z, A-Z und die ganzen anderen Tasten auch, außer Tab und so
  (:Pressed
    (if (Variables|Default|GetshiftClicked)
      (Class|WidgetInteractionComponent|SendKeyChar _widgetinteractionmouse "P" false)
      (else
        (Class|WidgetInteractionComponent|SendKeyChar _widgetinteractionmouse "p" false)))))

(event Input|KeyboardEvents|Delete
  (params (Key :type Key%20Structure :default "None"))
  (bind _widgetinteractionmouse (Variables|Default|GetWidgetInteractionMouse))
  ;[1 1 1] Backspace & Delete
  (:Pressed
    (Class|WidgetInteractionComponent|PressKey _widgetinteractionmouse "Delete" true))
  (:Released
    (Class|WidgetInteractionComponent|ReleaseKey _widgetinteractionmouse "Delete")))

(event Input|KeyboardEvents|Q
  (params (Key :type Key%20Structure :default "None"))
  (bind _widgetinteractionmouse (Variables|Default|GetWidgetInteractionMouse))
  ;[1 1 1] a-z, A-Z und die ganzen anderen Tasten auch, außer Tab und so
  (:Pressed
    (if (Variables|Default|GetshiftClicked)
      (Class|WidgetInteractionComponent|SendKeyChar _widgetinteractionmouse "Q" false)
      (else
        (Class|WidgetInteractionComponent|SendKeyChar _widgetinteractionmouse "q" false)))))

(event Input|KeyboardEvents|R
  (params (Key :type Key%20Structure :default "None"))
  (bind _widgetinteractionmouse (Variables|Default|GetWidgetInteractionMouse))
  ;[1 1 1] a-z, A-Z und die ganzen anderen Tasten auch, außer Tab und so
  (:Pressed
    (if (Variables|Default|GetshiftClicked)
      (Class|WidgetInteractionComponent|SendKeyChar _widgetinteractionmouse "R" false)
      (else
        (Class|WidgetInteractionComponent|SendKeyChar _widgetinteractionmouse "r" false)))))

(event Input|KeyboardEvents|S
  (params (Key :type Key%20Structure :default "None"))
  (bind _widgetinteractionmouse (Variables|Default|GetWidgetInteractionMouse))
  ;[1 1 1] a-z, A-Z und die ganzen anderen Tasten auch, außer Tab und so
  (:Pressed
    (if (Variables|Default|GetshiftClicked)
      (Class|WidgetInteractionComponent|SendKeyChar _widgetinteractionmouse "S" false)
      (else
        (Class|WidgetInteractionComponent|SendKeyChar _widgetinteractionmouse "s" false)))))

(event Input|KeyboardEvents|T
  (params (Key :type Key%20Structure :default "None"))
  (bind _widgetinteractionmouse (Variables|Default|GetWidgetInteractionMouse))
  ;[1 1 1] a-z, A-Z und die ganzen anderen Tasten auch, außer Tab und so
  (:Pressed
    (if (Variables|Default|GetshiftClicked)
      (Class|WidgetInteractionComponent|SendKeyChar _widgetinteractionmouse "T" false)
      (else
        (Class|WidgetInteractionComponent|SendKeyChar _widgetinteractionmouse "t" false)))))

(event Input|KeyboardEvents|U
  (params (Key :type Key%20Structure :default "None"))
  (bind _widgetinteractionmouse (Variables|Default|GetWidgetInteractionMouse))
  ;[1 1 1] a-z, A-Z und die ganzen anderen Tasten auch, außer Tab und so
  (:Pressed
    (if (Variables|Default|GetshiftClicked)
      (Class|WidgetInteractionComponent|SendKeyChar _widgetinteractionmouse "U" false)
      (else
        (Class|WidgetInteractionComponent|SendKeyChar _widgetinteractionmouse "u" false)))))

(event Input|KeyboardEvents|V
  (params (Key :type Key%20Structure :default "None"))
  (bind _widgetinteractionmouse (Variables|Default|GetWidgetInteractionMouse))
  ;[1 1 1] a-z, A-Z und die ganzen anderen Tasten auch, außer Tab und so
  (:Pressed
    (if (Variables|Default|GetshiftClicked)
      (Class|WidgetInteractionComponent|SendKeyChar _widgetinteractionmouse "V" false)
      (else
        (Class|WidgetInteractionComponent|SendKeyChar _widgetinteractionmouse "v" false)))))

(event Input|KeyboardEvents|W
  (params (Key :type Key%20Structure :default "None"))
  (bind _widgetinteractionmouse (Variables|Default|GetWidgetInteractionMouse))
  ;[1 1 1] a-z, A-Z und die ganzen anderen Tasten auch, außer Tab und so
  (:Pressed
    (if (Variables|Default|GetshiftClicked)
      (Class|WidgetInteractionComponent|SendKeyChar _widgetinteractionmouse "W" false)
      (else
        (Class|WidgetInteractionComponent|SendKeyChar _widgetinteractionmouse "w" false)))))

(event Input|KeyboardEvents|X
  (params (Key :type Key%20Structure :default "None"))
  (bind _widgetinteractionmouse (Variables|Default|GetWidgetInteractionMouse))
  ;[1 1 1] a-z, A-Z und die ganzen anderen Tasten auch, außer Tab und so
  (:Pressed
    (if (Variables|Default|GetshiftClicked)
      (Class|WidgetInteractionComponent|SendKeyChar _widgetinteractionmouse "X" false)
      (else
        (Class|WidgetInteractionComponent|SendKeyChar _widgetinteractionmouse "x" false)))))

(event Input|KeyboardEvents|Y
  (params (Key :type Key%20Structure :default "None"))
  (bind _widgetinteractionmouse (Variables|Default|GetWidgetInteractionMouse))
  ;[1 1 1] a-z, A-Z und die ganzen anderen Tasten auch, außer Tab und so
  (:Pressed
    (if (Variables|Default|GetshiftClicked)
      (Class|WidgetInteractionComponent|SendKeyChar _widgetinteractionmouse "Y" false)
      (else
        (Class|WidgetInteractionComponent|SendKeyChar _widgetinteractionmouse "y" false)))))

(event Input|KeyboardEvents|Z
  (params (Key :type Key%20Structure :default "None"))
  (bind _widgetinteractionmouse (Variables|Default|GetWidgetInteractionMouse))
  ;[1 1 1] a-z, A-Z und die ganzen anderen Tasten auch, außer Tab und so
  (:Pressed
    (if (Variables|Default|GetshiftClicked)
      (Class|WidgetInteractionComponent|SendKeyChar _widgetinteractionmouse "Z" false)
      (else
        (Class|WidgetInteractionComponent|SendKeyChar _widgetinteractionmouse "z" false)))))

(event Input|KeyboardEvents|RightShift
  (params (Key :type Key%20Structure :default "None"))
  ;[1 1 1] Toggle Shift
  (:Pressed
    (Variables|Default|SetshiftClicked true))
  (:Released
    (Variables|Default|SetshiftClicked false)))

(event Input|KeyboardEvents|Period
  (params (Key :type Key%20Structure :default "None"))
  (bind _widgetinteractionmouse (Variables|Default|GetWidgetInteractionMouse))
  ;[1 1 1] a-z, A-Z und die ganzen anderen Tasten auch, außer Tab und so
  (:Pressed
    (if (Variables|Default|GetshiftClicked)
      (Class|WidgetInteractionComponent|SendKeyChar _widgetinteractionmouse ":" false)
      (else
        (Class|WidgetInteractionComponent|SendKeyChar _widgetinteractionmouse "." false)))))

(event Input|KeyboardEvents|Comma
  (params (Key :type Key%20Structure :default "None"))
  (bind _widgetinteractionmouse (Variables|Default|GetWidgetInteractionMouse))
  ;[1 1 1] a-z, A-Z und die ganzen anderen Tasten auch, außer Tab und so
  (:Pressed
    (if (Variables|Default|GetshiftClicked)
      (Class|WidgetInteractionComponent|SendKeyChar _widgetinteractionmouse ";" false)
      (else
        (Class|WidgetInteractionComponent|SendKeyChar _widgetinteractionmouse "," false)))))

(event Input|KeyboardEvents|SpaceBar
  (params (Key :type Key%20Structure :default "None"))
  (bind _widgetinteractionmouse (Variables|Default|GetWidgetInteractionMouse))
  ;[1 1 1] a-z, A-Z und die ganzen anderen Tasten auch, außer Tab und so
  (:Pressed
    (if (Variables|Default|GetshiftClicked)
      (Class|WidgetInteractionComponent|SendKeyChar _widgetinteractionmouse "    " false)
      (else
        (Class|WidgetInteractionComponent|SendKeyChar _widgetinteractionmouse " " false)))))

(event Input|KeyboardEvents|Ü
  (params (Key :type Key%20Structure :default "None"))
  (bind _widgetinteractionmouse (Variables|Default|GetWidgetInteractionMouse))
  ;[1 1 1] a-z, A-Z und die ganzen anderen Tasten auch, außer Tab und so
  (:Pressed
    (if (Variables|Default|GetshiftClicked)
      (Class|WidgetInteractionComponent|SendKeyChar _widgetinteractionmouse "Ü" false)
      (else
        (Class|WidgetInteractionComponent|SendKeyChar _widgetinteractionmouse "ü" false)))))

(event Input|KeyboardEvents|<
  (params (Key :type Key%20Structure :default "None"))
  (bind _widgetinteractionmouse (Variables|Default|GetWidgetInteractionMouse))
  ;[1 1 1] a-z, A-Z und die ganzen anderen Tasten auch, außer Tab und so
  (:Pressed
    (if (Variables|Default|GetshiftClicked)
      (Class|WidgetInteractionComponent|SendKeyChar _widgetinteractionmouse ">" false)
      (else
        (Class|WidgetInteractionComponent|SendKeyChar _widgetinteractionmouse "<" false)))))

(event Input|KeyboardEvents|^
  (params (Key :type Key%20Structure :default "None"))
  (bind _widgetinteractionmouse (Variables|Default|GetWidgetInteractionMouse))
  ;[1 1 1] a-z, A-Z und die ganzen anderen Tasten auch, außer Tab und so
  (:Pressed
    (if (Variables|Default|GetshiftClicked)
      (Class|WidgetInteractionComponent|SendKeyChar _widgetinteractionmouse "°" false)
      (else
        (Class|WidgetInteractionComponent|SendKeyChar _widgetinteractionmouse "^" false)))))

(event Input|KeyboardEvents|0
  (params (Key :type Key%20Structure :default "None"))
  (bind _widgetinteractionmouse (Variables|Default|GetWidgetInteractionMouse))
  ;[1 1 1] 0-9, !-=
  (:Pressed
    (if (Variables|Default|GetshiftClicked)
      (Class|WidgetInteractionComponent|SendKeyChar _widgetinteractionmouse "=" false)
      (else
        (Class|WidgetInteractionComponent|SendKeyChar _widgetinteractionmouse "0" false)))))

(event Input|KeyboardEvents|NumPadZero
  (params (Key :type Key%20Structure :default "None"))
  ;[1 1 1] 0-9, !-=
  (:Pressed
    (Class|WidgetInteractionComponent|SendKeyChar (Variables|Default|GetWidgetInteractionMouse) "0" false)))

(event Input|KeyboardEvents|NumPadOne
  (params (Key :type Key%20Structure :default "None"))
  ;[1 1 1] 0-9, !-=
  (:Pressed
    (Class|WidgetInteractionComponent|SendKeyChar (Variables|Default|GetWidgetInteractionMouse) "1" false)))

(event Input|KeyboardEvents|NumPadTwo
  (params (Key :type Key%20Structure :default "None"))
  ;[1 1 1] 0-9, !-=
  (:Pressed
    (Class|WidgetInteractionComponent|SendKeyChar (Variables|Default|GetWidgetInteractionMouse) "2" false)))

(event Input|KeyboardEvents|2
  (params (Key :type Key%20Structure :default "None"))
  (bind _widgetinteractionmouse (Variables|Default|GetWidgetInteractionMouse))
  ;[1 1 1] 0-9, !-=
  (:Pressed
    (if (Variables|Default|GetshiftClicked)
      (Class|WidgetInteractionComponent|SendKeyChar _widgetinteractionmouse "\"" false)
      (else
        (Class|WidgetInteractionComponent|SendKeyChar _widgetinteractionmouse "2" false)))))

(event Input|KeyboardEvents|NumPadThree
  (params (Key :type Key%20Structure :default "None"))
  ;[1 1 1] 0-9, !-=
  (:Pressed
    (Class|WidgetInteractionComponent|SendKeyChar (Variables|Default|GetWidgetInteractionMouse) "3" false)))

(event Input|KeyboardEvents|NumPadFour
  (params (Key :type Key%20Structure :default "None"))
  ;[1 1 1] 0-9, !-=
  (:Pressed
    (Class|WidgetInteractionComponent|SendKeyChar (Variables|Default|GetWidgetInteractionMouse) "4" false)))

(event Input|KeyboardEvents|NumPadFive
  (params (Key :type Key%20Structure :default "None"))
  ;[1 1 1] 0-9, !-=
  (:Pressed
    (Class|WidgetInteractionComponent|SendKeyChar (Variables|Default|GetWidgetInteractionMouse) "5" false)))

(event Input|KeyboardEvents|NumPadSix
  (params (Key :type Key%20Structure :default "None"))
  ;[1 1 1] 0-9, !-=
  (:Pressed
    (Class|WidgetInteractionComponent|SendKeyChar (Variables|Default|GetWidgetInteractionMouse) "6" false)))

(event Input|KeyboardEvents|NumPadSeven
  (params (Key :type Key%20Structure :default "None"))
  ;[1 1 1] 0-9, !-=
  (:Pressed
    (Class|WidgetInteractionComponent|SendKeyChar (Variables|Default|GetWidgetInteractionMouse) "7" false)))

(event Input|KeyboardEvents|NumPadEight
  (params (Key :type Key%20Structure :default "None"))
  ;[1 1 1] 0-9, !-=
  (:Pressed
    (Class|WidgetInteractionComponent|SendKeyChar (Variables|Default|GetWidgetInteractionMouse) "8" false)))

(event Input|KeyboardEvents|SS
  (params (Key :type Key%20Structure :default "None"))
  (bind _widgetinteractionmouse (Variables|Default|GetWidgetInteractionMouse))
  ;[1 1 1] a-z, A-Z und die ganzen anderen Tasten auch, außer Tab und so
  (:Pressed
    (if (Variables|Default|GetshiftClicked)
      (Class|WidgetInteractionComponent|SendKeyChar _widgetinteractionmouse "?" false)
      (else
        (Class|WidgetInteractionComponent|SendKeyChar _widgetinteractionmouse "ß" false)))))

(event Input|KeyboardEvents|+
  (params (Key :type Key%20Structure :default "None"))
  (bind _widgetinteractionmouse (Variables|Default|GetWidgetInteractionMouse))
  ;[1 1 1] a-z, A-Z und die ganzen anderen Tasten auch, außer Tab und so
  (:Pressed
    (if (Variables|Default|GetshiftClicked)
      (Class|WidgetInteractionComponent|SendKeyChar _widgetinteractionmouse "*" false)
      (else
        (Class|WidgetInteractionComponent|SendKeyChar _widgetinteractionmouse "+" false)))))

(event Input|KeyboardEvents|LeftShift
  (params (Key :type Key%20Structure :default "None"))
  ;[1 1 1] Toggle Shift
  (:Pressed
    (Variables|Default|SetshiftClicked true))
  (:Released
    (Variables|Default|SetshiftClicked false)))

(event Input|KeyboardEvents|CapsLock
  (params (Key :type Key%20Structure :default "None"))
  ;[1 1 1] Capslock
  (:Pressed
    (Variables|Default|SetshiftClicked (not (Variables|Default|GetshiftClicked)))))

(event Input|KeyboardEvents|3
  (params (Key :type Key%20Structure :default "None"))
  (bind _widgetinteractionmouse (Variables|Default|GetWidgetInteractionMouse))
  ;[1 1 1] 0-9, !-=
  (:Pressed
    (if (Variables|Default|GetshiftClicked)
      (Class|WidgetInteractionComponent|SendKeyChar _widgetinteractionmouse "§" false)
      (else
        (Class|WidgetInteractionComponent|SendKeyChar _widgetinteractionmouse "3" false)))))

(event Input|KeyboardEvents|Backspace
  (params (Key :type Key%20Structure :default "None"))
  (bind _widgetinteractionmouse (Variables|Default|GetWidgetInteractionMouse))
  ;[1 1 1] Backspace & Delete
  (:Pressed
    (Class|WidgetInteractionComponent|PressandReleaseKey _widgetinteractionmouse "BackSpace"))
  (:Released
    (Class|WidgetInteractionComponent|ReleaseKey _widgetinteractionmouse "BackSpace")))

(event Input|KeyboardEvents|Hyphen
  (params (Key :type Key%20Structure :default "None"))
  (bind _widgetinteractionmouse (Variables|Default|GetWidgetInteractionMouse))
  ;[1 1 1] a-z, A-Z und die ganzen anderen Tasten auch, außer Tab und so
  (:Pressed
    (if (Variables|Default|GetshiftClicked)
      (Class|WidgetInteractionComponent|SendKeyChar _widgetinteractionmouse "_" false)
      (else
        (Class|WidgetInteractionComponent|SendKeyChar _widgetinteractionmouse "-" false)))))

(event Input|KeyboardEvents|Ä
  (params (Key :type Key%20Structure :default "None"))
  (bind _widgetinteractionmouse (Variables|Default|GetWidgetInteractionMouse))
  ;[1 1 1] a-z, A-Z und die ganzen anderen Tasten auch, außer Tab und so
  (:Pressed
    (if (Variables|Default|GetshiftClicked)
      (Class|WidgetInteractionComponent|SendKeyChar _widgetinteractionmouse "Ä" false)
      (else
        (Class|WidgetInteractionComponent|SendKeyChar _widgetinteractionmouse "ä" false)))))

(event Input|KeyboardEvents|Ö
  (params (Key :type Key%20Structure :default "None"))
  (bind _widgetinteractionmouse (Variables|Default|GetWidgetInteractionMouse))
  ;[1 1 1] a-z, A-Z und die ganzen anderen Tasten auch, außer Tab und so
  (:Pressed
    (if (Variables|Default|GetshiftClicked)
      (Class|WidgetInteractionComponent|SendKeyChar _widgetinteractionmouse "Ö" false)
      (else
        (Class|WidgetInteractionComponent|SendKeyChar _widgetinteractionmouse "ö" false)))))

(event Input|KeyboardEvents|4
  (params (Key :type Key%20Structure :default "None"))
  (bind _widgetinteractionmouse (Variables|Default|GetWidgetInteractionMouse))
  ;[1 1 1] 0-9, !-=
  (:Pressed
    (if (Variables|Default|GetshiftClicked)
      (Class|WidgetInteractionComponent|SendKeyChar _widgetinteractionmouse "$" false)
      (else
        (Class|WidgetInteractionComponent|SendKeyChar _widgetinteractionmouse "4" false)))))

(event Input|KeyboardEvents|5
  (params (Key :type Key%20Structure :default "None"))
  (bind _widgetinteractionmouse (Variables|Default|GetWidgetInteractionMouse))
  ;[1 1 1] 0-9, !-=
  (:Pressed
    (if (Variables|Default|GetshiftClicked)
      (Class|WidgetInteractionComponent|SendKeyChar _widgetinteractionmouse "%" false)
      (else
        (Class|WidgetInteractionComponent|SendKeyChar _widgetinteractionmouse "5" false)))))

(event Input|KeyboardEvents|6
  (params (Key :type Key%20Structure :default "None"))
  (bind _widgetinteractionmouse (Variables|Default|GetWidgetInteractionMouse))
  ;[1 1 1] 0-9, !-=
  (:Pressed
    (if (Variables|Default|GetshiftClicked)
      (Class|WidgetInteractionComponent|SendKeyChar _widgetinteractionmouse "&" false)
      (else
        (Class|WidgetInteractionComponent|SendKeyChar _widgetinteractionmouse "6" false)))))

(fn ConstructionScript)

(fn InputCharacter
  (params (Character :type Character%20Event%20Structure) (ShiftClicked :type Boolean)))