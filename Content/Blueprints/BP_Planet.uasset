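; Planet actor that holds PlanetState, a struct of per-continent arrays for population, energy mix, climate and grid cell counts.
; Init helpers seed the first continent from the save's population preset and zero-fill others, but their save-loading chain is unwired.
; Power plant and city functions update cell counts and plant tallies by type and tier, with nuclear occupying nine cells.
; BeginPlay only prints a debug cell count; Tick is empty.
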(event EventBeginPlay
  (Utilities|FlowControl|Delay 0 0.02)
  (Development|PrintString 0 (Utilities|String|ToString(Integer) (Variables|Default|GetglobalUsableCellCount self)) true true "(R=0.000000,G=0.660000,B=1.000000,A=1.000000)" 2e+01))

(event Collision|EventActorBeginOverlap
  (params (OtherActor :type Actor%20Object%20Reference)))

(event EventTick
  (params (DeltaSeconds :type Float%20%28single-precision%29)))

(fn ConstructionScript)

(fn Init)

(fn InitPopulation
  (params (SaveGame :type Save%20Game%20Object%20Reference))
  (switch string (Variables|/Game/SaveGame/SaveGame.SaveGame_C|GetPopulation SaveGame)
    (:Default
      ;[1 1 1] Bad Style
      (LocalVariables|SetPopulation 1e+03 :!label _label)
      (LocalVariables|SetGrowthRate 1.015)
      (LocalVariables|SetDeathRate 1.01))
    (:Underpopulated
      (LocalVariables|SetPopulation 1e+02)
      (LocalVariables|SetGrowthRate 1.01)
      (LocalVariables|SetDeathRate 1.011))
    (:Self%20Sustaining
      (goto _label))
    (:Crowded
      (LocalVariables|SetPopulation 1e+04)
      (LocalVariables|SetGrowthRate 1.018)
      (LocalVariables|SetDeathRate 1.01))
    (:Overpopulated
      (LocalVariables|SetPopulation 1e+05)
      (LocalVariables|SetGrowthRate 1.02)
      (LocalVariables|SetDeathRate 1.012)))
  ;[1 1 1] Start Continent
  (Utilities|Array|Add (.population (Variables|Default|GetPlanetState)) (LocalVariables|GetPopulation))
  (Utilities|Array|Add (.populationgrowth (Variables|Default|GetPlanetState)) (LocalVariables|GetGrowthRate))
  (Utilities|Array|Add (.deathrate (Variables|Default|GetPlanetState)) (LocalVariables|GetDeathRate))
  (Utilities|Array|Add (.populationworkforce (Variables|Default|GetPlanetState)) (* (LocalVariables|GetPopulation) (Variables|Default|GetWorkForceMP)))
  (Utilities|Array|Add (.energypercapita (Variables|Default|GetPlanetState)) 3081)
  (bind _index (Utilities|FlowControl|ForLoopwithBreak 1 (- (Variables|Default|GetNumContinents) 1))
    (:LoopBody
      ;[1 1 1] Fill Zeroes
      (Utilities|Array|Insert (.population (Variables|Default|GetPlanetState)) 0.0 _index)
      (Utilities|Array|Insert (.populationgrowth (Variables|Default|GetPlanetState)) 0.0 _index)
      (Utilities|Array|Insert (.deathrate (Variables|Default|GetPlanetState)) 0.0 _index)
      (Utilities|Array|Insert (.populationworkforce (Variables|Default|GetPlanetState)) 0.0 _index)
      (Utilities|Array|Insert (.energypercapita (Variables|Default|GetPlanetState)) 0 _index))
    (:Completed
      (Variables|Default|SetPlanetState (Utilities|Struct|MakePlanetState (.gridcells (Variables|Default|GetPlanetState)) (.usablecells (Variables|Default|GetPlanetState)) (.unusablecells (Variables|Default|GetPlanetState)) (.occupiedcells (Variables|Default|GetPlanetState)) (.plantcells (Variables|Default|GetPlanetState)) (.citycells (Variables|Default|GetPlanetState)) (.population (Variables|Default|GetPlanetState)) (.populationgrowth (Variables|Default|GetPlanetState)) (.deathrate (Variables|Default|GetPlanetState)) (.populationenergyconsumption (Variables|Default|GetPlanetState)) (.populationworkforce (Variables|Default|GetPlanetState)) (.climateaffection (Variables|Default|GetPlanetState)) (.co2level (Variables|Default|GetPlanetState)) (.temperaturincrease (Variables|Default|GetPlanetState)) (.energygenerationtotal (Variables|Default|GetPlanetState)) (.usablesurface (Variables|Default|GetPlanetState)) (.ressources (Variables|Default|GetPlanetState)) (.month (Variables|Default|GetPlanetState)) (Variables|Default|GetStartYear) (.energymix (Variables|Default|GetPlanetState)) (.energypercapita (Variables|Default|GetPlanetState)) (Variables|Default|GetNumContinents))))))

(fn InitEnergy
  (params (SaveGame :type Save%20Game%20Object%20Reference))
  (bind _emix (Variables|Default|GetEMix))
  (Utilities|Array|Insert (.populationenergyconsumption (Variables|Default|GetPlanetState)) 0.0)
  (Utilities|Array|Insert (.energygenerationtotal (Variables|Default|GetPlanetState)) 0.0)
  ;[1 1 1] Start Continent
  (Utilities|Array|Insert (.energymix (Variables|Default|GetPlanetState)) _emix)
  (bind _index (Utilities|FlowControl|ForLoopwithBreak 1 (- (Variables|Default|GetNumContinents) 1))
    (:LoopBody
      ;[1 1 1] Fill Zeroes
      (Utilities|Array|Insert (.energymix (Variables|Default|GetPlanetState)) _emix _index)
      (Utilities|Array|Insert (.populationenergyconsumption (Variables|Default|GetPlanetState)) 0.0 _index)
      (Utilities|Array|Insert (.energygenerationtotal (Variables|Default|GetPlanetState)) 0.0 _index))
    (:Completed
      (Variables|Default|SetPlanetState (Utilities|Struct|MakePlanetState (.gridcells (Variables|Default|GetPlanetState)) (.usablecells (Variables|Default|GetPlanetState)) (.unusablecells (Variables|Default|GetPlanetState)) (.occupiedcells (Variables|Default|GetPlanetState)) (.plantcells (Variables|Default|GetPlanetState)) (.citycells (Variables|Default|GetPlanetState)) (.population (Variables|Default|GetPlanetState)) (.populationgrowth (Variables|Default|GetPlanetState)) (.deathrate (Variables|Default|GetPlanetState)) (.populationenergyconsumption (Variables|Default|GetPlanetState)) (.populationworkforce (Variables|Default|GetPlanetState)) (.climateaffection (Variables|Default|GetPlanetState)) (.co2level (Variables|Default|GetPlanetState)) (.temperaturincrease (Variables|Default|GetPlanetState)) (.energygenerationtotal (Variables|Default|GetPlanetState)) (.usablesurface (Variables|Default|GetPlanetState)) (.ressources (Variables|Default|GetPlanetState)) (.month (Variables|Default|GetPlanetState)) (Variables|Default|GetStartYear) (.energymix (Variables|Default|GetPlanetState)) (.energypercapita (Variables|Default|GetPlanetState)) (Variables|Default|GetNumContinents))))))

(fn InitCells
  (bind _planetstate (Variables|Default|GetPlanetState))
  (for _index (range 0 (- (.continents _planetstate) 1))
    (LocalVariables|Setunusable 0)
    (LocalVariables|Setusable 0)
    (bind _output_get (LocalVariables|SetTotal (+ 0 1)))
    (Utilities|Array|Insert (.gridcells _planetstate) _output_get _index)
    (Utilities|Array|Insert (.usablecells _planetstate) (LocalVariables|Getunusable) _index)
    (Utilities|Array|Insert (.unusablecells _planetstate) (LocalVariables|Getunusable) _index)
    (Utilities|Array|Insert (.occupiedcells _planetstate) 0 _index)
    (Utilities|Array|Insert (.plantcells _planetstate) 0 _index)
    (Utilities|Array|Insert (.citycells _planetstate) 0 _index)))

(fn InitClimate
  ;[1 1 1] Start Continent
  (Utilities|Array|Insert (.climateaffection (Variables|Default|GetPlanetState)) 0)
  (Utilities|Array|Insert (.co2level (Variables|Default|GetPlanetState)) 0)
  (Utilities|Array|Insert (.temperaturincrease (Variables|Default|GetPlanetState)) 0.0)
  (bind _index (Utilities|FlowControl|ForLoopwithBreak 1 (- (Variables|Default|GetNumContinents) 1))
    (:LoopBody
      ;[1 1 1] Fill Zeroes
      (Utilities|Array|Insert (.climateaffection (Variables|Default|GetPlanetState)) 0 _index)
      (Utilities|Array|Insert (.co2level (Variables|Default|GetPlanetState)) 0 _index)
      (Utilities|Array|Insert (.temperaturincrease (Variables|Default|GetPlanetState)) 0.0 _index))
    (:Completed
      (Variables|Default|SetPlanetState (Utilities|Struct|MakePlanetState (.gridcells (Variables|Default|GetPlanetState)) (.usablecells (Variables|Default|GetPlanetState)) (.unusablecells (Variables|Default|GetPlanetState)) (.occupiedcells (Variables|Default|GetPlanetState)) (.plantcells (Variables|Default|GetPlanetState)) (.citycells (Variables|Default|GetPlanetState)) (.population (Variables|Default|GetPlanetState)) (.populationgrowth (Variables|Default|GetPlanetState)) (.deathrate (Variables|Default|GetPlanetState)) (.populationenergyconsumption (Variables|Default|GetPlanetState)) (.populationworkforce (Variables|Default|GetPlanetState)) (.climateaffection (Variables|Default|GetPlanetState)) (.co2level (Variables|Default|GetPlanetState)) (.temperaturincrease (Variables|Default|GetPlanetState)) (.energygenerationtotal (Variables|Default|GetPlanetState)) (.usablesurface (Variables|Default|GetPlanetState)) (.ressources (Variables|Default|GetPlanetState)) (.month (Variables|Default|GetPlanetState)) (Variables|Default|GetStartYear) (.energymix (Variables|Default|GetPlanetState)) (.energypercapita (Variables|Default|GetPlanetState)) (Variables|Default|GetNumContinents))))))

(fn AddorActivatePowerPlant
  (params (Type :type String) (Tier :type Integer) (ContinentID :type Integer))
  (bind _planetstate (Variables|Default|GetPlanetState))
  (bind _planetstate_2 (Variables|Default|GetPlanetState))
  (bind _planetstate_3 (Variables|Default|GetPlanetState))
  (bind _output (Utilities|Array|Get(acopy) (.energymix _planetstate_2) ContinentID))
  (bind _result (Math|Integer|IncrementInt (Utilities|Array|Get(acopy) (.plantcells _planetstate) ContinentID))
    (:%20%20
      (Utilities|Array|SetArrayElem (.plantcells _planetstate) ContinentID _result)
      (switch string Type
        (:Oil
          (bind _result_2 (Math|Integer|DecrementInt (Utilities|Array|Get(acopy) (.usablecells _planetstate_3) ContinentID) :!label _label)
            (:%20%20
              (Utilities|Array|SetArrayElem (.usablecells _planetstate_3) ContinentID _result_2)
              (bind _result_3 (Math|Integer|IncrementInt (Utilities|Array|Get(acopy) (.occupiedcells _planetstate_3) ContinentID))
                (:%20%20
                  (Utilities|Array|SetArrayElem (.occupiedcells _planetstate_3) ContinentID _result_3))))))
        (:Coal
          (goto _label))
        (:Gas
          (goto _label))
        (:Nuclear
          (Utilities|Array|SetArrayElem (.usablecells _planetstate_3) ContinentID (- (Utilities|Array|Get(acopy) (.usablecells _planetstate_3) ContinentID) 9))
          (Utilities|Array|SetArrayElem (.occupiedcells _planetstate_3) ContinentID (+ (Utilities|Array|Get(acopy) (.occupiedcells _planetstate_3) ContinentID) 9)))
        (:Hydro
          (goto _label))
        (:Wind
          (goto _label))
        (:Solar
          (goto _label))
        (:BioFuel
          (goto _label)))
      (bind _result_4 (Math|Integer|IncrementInt (Utilities|Array|Get(acopy) (.plantcells _planetstate_3) ContinentID))
        (:%20%20
          (Utilities|Array|SetArrayElem (.plantcells _planetstate_3) ContinentID _result_4)
          (switch string Type
            (:Oil
              (Math|Integer|IncrementInt (Utilities|Array|Get(acopy) (.oil _output) Tier)))
            (:Coal
              (Math|Integer|IncrementInt (Utilities|Array|Get(acopy) (.coal _output) Tier)))
            (:Gas
              (Math|Integer|IncrementInt (Utilities|Array|Get(acopy) (.gas _output) Tier)))
            (:Nuclear
              (Math|Integer|IncrementInt (Utilities|Array|Get(acopy) (.nuclear _output) Tier)))
            (:Hydro
              (Math|Integer|IncrementInt (Utilities|Array|Get(acopy) (.hydro _output) Tier)))
            (:Wind
              (Math|Integer|IncrementInt (Utilities|Array|Get(acopy) (.wind _output) Tier)))
            (:Solar
              (Math|Integer|IncrementInt (Utilities|Array|Get(acopy) (.solar _output) Tier)))
            (:BioFuel
              (Math|Integer|IncrementInt (Utilities|Array|Get(acopy) (.biofuel _output) Tier)))))))))

(fn AddCity
  (params (CityPieces :type Integer) (ContinentID :type Integer))
  (bind _planetstate (Variables|Default|GetPlanetState))
  (bind _result (Math|Integer|DecrementInt (Utilities|Array|Get(acopy) (.usablecells _planetstate) ContinentID))
    (:%20%20
      (Utilities|Array|SetArrayElem (.usablecells _planetstate) ContinentID _result)
      (bind _result_2 (Math|Integer|IncrementInt (Utilities|Array|Get(acopy) (.occupiedcells _planetstate) ContinentID))
        (:%20%20
          (Utilities|Array|SetArrayElem (.occupiedcells _planetstate) ContinentID _result_2)
          (bind _result_3 (Math|Integer|IncrementInt (Utilities|Array|Get(acopy) (.citycells _planetstate) ContinentID))
            (:%20%20
              (Utilities|Array|SetArrayElem (.citycells _planetstate) ContinentID _result_3))))))))

(fn DisablePowerPlant
  (params (Type :type String) (Tier :type Integer) (ContinentID :type Integer))
  (bind _planetstate (Variables|Default|GetPlanetState))
  (bind _output (Utilities|Array|Get(acopy) (.energymix _planetstate) ContinentID))
  (switch string Type
    (:Oil
      (Math|Integer|DecrementInt (Utilities|Array|Get(acopy) (.oil _output) Tier)))
    (:Coal
      (Math|Integer|DecrementInt (Utilities|Array|Get(acopy) (.coal _output) Tier)))
    (:Gas
      (Math|Integer|DecrementInt (Utilities|Array|Get(acopy) (.gas _output) Tier)))
    (:Nuclear
      (Math|Integer|DecrementInt (Utilities|Array|Get(acopy) (.nuclear _output) Tier)))
    (:Hydro
      (Math|Integer|DecrementInt (Utilities|Array|Get(acopy) (.hydro _output) Tier)))
    (:Wind
      (Math|Integer|DecrementInt (Utilities|Array|Get(acopy) (.wind _output) Tier)))
    (:Solar
      (Math|Integer|DecrementInt (Utilities|Array|Get(acopy) (.solar _output) Tier)))
    (:BioFuel
      (Math|Integer|DecrementInt (Utilities|Array|Get(acopy) (.biofuel _output) Tier)))))

(fn ReactivatePowerPlant
  (params (Type :type String) (Tier :type Integer) (ContinentID :type Integer))
  (bind _planetstate (Variables|Default|GetPlanetState))
  (bind _output (Utilities|Array|Get(acopy) (.energymix _planetstate) ContinentID))
  (switch string Type
    (:Oil
      (Math|Integer|IncrementInt (Utilities|Array|Get(acopy) (.oil _output) Tier)))
    (:Coal
      (Math|Integer|IncrementInt (Utilities|Array|Get(acopy) (.coal _output) Tier)))
    (:Gas
      (Math|Integer|IncrementInt (Utilities|Array|Get(acopy) (.gas _output) Tier)))
    (:Nuclear
      (Math|Integer|IncrementInt (Utilities|Array|Get(acopy) (.nuclear _output) Tier)))
    (:Hydro
      (Math|Integer|IncrementInt (Utilities|Array|Get(acopy) (.hydro _output) Tier)))
    (:Wind
      (Math|Integer|IncrementInt (Utilities|Array|Get(acopy) (.wind _output) Tier)))
    (:Solar
      (Math|Integer|IncrementInt (Utilities|Array|Get(acopy) (.solar _output) Tier)))
    (:BioFuel
      (Math|Integer|IncrementInt (Utilities|Array|Get(acopy) (.biofuel _output) Tier)))))

(fn ScaleEnergyMix
  (Variables|Default|SetEMix (Utilities|Struct|MakeEnergyMix (.oil (Variables|Default|GetEMix)) (.coal (Variables|Default|GetEMix)) (.gas (Variables|Default|GetEMix)) (.nuclear (Variables|Default|GetEMix)) (.hydro (Variables|Default|GetEMix)) (.wind (Variables|Default|GetEMix)) (.solar (Variables|Default|GetEMix)) (.biofuel (Variables|Default|GetEMix)) (* (Variables|Default|GetPlantScaler) (.oilpower (Variables|Default|GetEMix))) (* (Variables|Default|GetPlantScaler) (.coalpower (Variables|Default|GetEMix))) (* (Variables|Default|GetPlantScaler) (.gaspower (Variables|Default|GetEMix))) (* (Variables|Default|GetPlantScaler) (.nuclearpower (Variables|Default|GetEMix))) (* (Variables|Default|GetPlantScaler) (.hydropower (Variables|Default|GetEMix))) (* (Variables|Default|GetPlantScaler) (.windpower (Variables|Default|GetEMix))) (* (Variables|Default|GetPlantScaler) (.solarpower (Variables|Default|GetEMix))) (* (Variables|Default|GetPlantScaler) (.biofuelpower (Variables|Default|GetEMix))) (.oilco2 (Variables|Default|GetEMix)) (.coalco2 (Variables|Default|GetEMix)) (.gasco2 (Variables|Default|GetEMix)) (.nuclearco2 (Variables|Default|GetEMix)) (.hydroco2 (Variables|Default|GetEMix)) (.windco2 (Variables|Default|GetEMix)) (.solarco2 (Variables|Default|GetEMix)) (.biofuelco2 (Variables|Default|GetEMix)))))