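; BP_Player is the player's orbit camera for viewing a PlanetGeneration planet.
; On BeginPlay it retries on a short delay until it finds the planet, then moves the spring arm to its center and sets the socket's X offset to the planet's radius.
; While Alt+right mouse is held, mouse movement drives controller yaw and pitch to rotate the view.
; The mouse wheel zooms by adjusting camera FOV within clamped limits.
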(event EventBeginPlay
  (bind _springarm (Variables|Default|GetSpringArm))
  (bind _outactors (Actor|GetAllActorsOfClass "/Game/PlanetGeneration.PlanetGeneration_C" :!label _label))
  (if (Utilities|IsValid (Utilities|Array|Get(acopy) _outactors))
    (bind _output_get (Variables|Default|SetPlanet (Utilities|Array|Get(acopy) _outactors)))
    (Transformation|SetWorldLocation _springarm (Transformation|GetWorldLocation (Variables|/Script/Engine.Actor|GetRootComponent _output_get)) false false)
    (Variables|/Script/Engine.SpringArmComponent|SetSocketOffset _springarm (Math|Vector|MakeVector (Math|Conversions|ToFloat(Integer) (Variables|/Script/MyProject2.MyActor|Getradius _output_get)) 0.0 0.0))
    (else
      (Utilities|FlowControl|Delay 0.2)
      (goto _label))))

(event Collision|EventActorBeginOverlap
  (params (OtherActor :type Actor%20Object%20Reference)))

(event EventTick
  (params (DeltaSeconds :type Float%20%28single-precision%29)))

(event Input|MouseEvents|MouseX
  (params (AxisValue :type Float%20%28single-precision%29))
  (bind _returnvalue (Game|GetPlayerController 0))
  (bind _returnvalue_2 (Pawn|GetControlRotation _returnvalue :!class /Script/Engine.Controller))
  ;[1 1 1] Rotation around planet
  (if (Variables|Default|GetRMBpressed)
    (Pawn|Input|AddControllerYawInput AxisValue)
    (Pawn|SetControlRotation _returnvalue (Math|Rotator|MakeRotator 0.0 (.pitch _returnvalue_2) (.yaw _returnvalue_2)))))

(event Input|MouseEvents|MouseY
  (params (AxisValue :type Float%20%28single-precision%29))
  ;[1 1 1] Rotation around planet
  (if (Variables|Default|GetRMBpressed)
    (Pawn|Input|AddControllerPitchInput AxisValue)))

(event Input|KeyboardEvents|S
  (params (Key :type Key%20Structure))
  ;[1 1 1] Rotation around planet
)

(event Input|MouseEvents|MouseWheelUp
  (params (Key :type Key%20Structure))
  (bind _camera (Variables|Default|GetCamera))
  ;[1 1 1] ZOOM in and out
  (:Pressed
    (Camera|SetFieldOfView _camera (Math|Float|Clamp(Float) (- (Variables|/Script/Engine.CameraComponent|GetFieldOfView _camera) 2.0) 3e+01 1.2e+02))))

(event Input|MouseEvents|MouseWheelDown
  (params (Key :type Key%20Structure))
  (bind _camera (Variables|Default|GetCamera))
  ;[1 1 1] ZOOM in and out
  (:Pressed
    (Camera|SetFieldOfView _camera (Math|Float|Clamp(Float) (+ (Variables|/Script/Engine.CameraComponent|GetFieldOfView _camera) 2.0) 3e+01 1.2e+02))))

(event Input|MouseEvents|AltRightMouseButton
  (params (Key :type Key%20Structure))
  ;[1 1 1] Rotation around planet
  (:Pressed
    (Variables|Default|SetRMBpressed true))
  (:Released
    (Variables|Default|SetRMBpressed false)))

(fn ConstructionScript)