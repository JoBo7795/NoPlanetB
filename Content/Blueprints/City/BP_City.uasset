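; City actor for a planet that players can click to select and show its info widget, unless it is display-only.
; Construction finds the PlanetGeneration actor, picks a mesh by tier and solar flag, and randomizes rotation in quarter turns; BeginPlay records the selected continent's index.
; Clicks clear every city's "Selector" material highlight, then FlipFlop this city's highlight and UI_CityInfo.
; Upgrade functions raise the tier or swap in solar meshes, setting the "ONOFF" material parameter.
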(event OnClicked(ClickAble)
  (params (TouchedComponent :type Primitive%20Component%20Object%20Reference) (ButtonPressed :type Key%20Structure))
  (bind _self self)
  (bind _citypiece (Variables|Default|GetCityPiece))
  (bind _widget (Variables|Default|GetWidget))
  (bind _returnvalue (UserInterface|GetWidget _widget))
  (bind _asui_city_info (Utilities|Casting|CastToUI_CityInfo _returnvalue))
  (if (not (Variables|Default|GetisDisplayOnly))
    (bind _outactors (Actor|GetAllActorsOfClass "BP_City_C"))
    (for _array_element _outactors
      (Rendering|Material|SetScalarParameterValueonMaterials (Variables|/Game/Blueprints/City/BP_City_Piece.BP_City_Piece_C|GetCityPiece _array_element) "Selector" 0.0))
    (Utilities|FlowControl|FlipFlop
      (:A
        (if true
          (UserInterface|Viewport|AddtoViewport _asui_city_info 0)
          (Variables|/Game/UI/UI_CityInfo.UI_CityInfo_C|SetOwner _asui_city_info _self)
          (Variables|Default|Setactive_0 true)
          (Rendering|Material|SetScalarParameterValueonMaterials _citypiece "Selector" 1.0)
          (else
            (Development|PrintString "CAST FAILED"))))
      (:B
        (Widget|RemovefromParent _asui_city_info)
        (Variables|/Game/UI/UI_CityInfo.UI_CityInfo_C|SetOwner _asui_city_info _self)
        (Variables|Default|Setactive_0 false)
        (Rendering|Material|SetScalarParameterValueonMaterials _citypiece "Selector" 0.0)))))

(event EventBeginPlay
  (bind _planet (Variables|Default|GetPlanet))
  (if (not (Variables|Default|GetisDisplayOnly))
    (bind _returnvalue (Class|MyActor|GetSelectedContinentID _planet))
    (Variables|Default|Setorigin (Utilities|Array|FindItem (Variables|/Game/PlanetGeneration.PlanetGeneration_C|GetContinentIDs _planet) _returnvalue))))

(event Collision|EventActorBeginOverlap
  (params (OtherActor :type Actor%20Object%20Reference))
  (|CallParentFunction OtherActor) ; This node is disabled and will not be called.\nDrag off pins to build functionality.
)

(event EventTick
  (params (DeltaSeconds :type Float%20%28single-precision%29))
  (|CallParentFunction DeltaSeconds) ; This node is disabled and will not be called.\nDrag off pins to build functionality.
)

(fn ConstructionScript
  (bind _outactors (Actor|GetAllActorsOfClass "/Game/PlanetGeneration.PlanetGeneration_C"))
  (if (Utilities|IsValid (Utilities|Array|Get(acopy) _outactors))
    (Variables|Default|SetPlanet (Utilities|Array|Get(acopy) _outactors))
    (switch int (Variables|Default|GetType)
      (:0
        (if (Variables|Default|GetisSolarPowered)
          (Components|StaticMesh|SetStaticMesh (Variables|Default|GetCityPiece) "/Game/Geometry/Meshes/City/SM_City_0_Solar.SM_City_0_Solar")
          (else
            (Components|StaticMesh|SetStaticMesh (Variables|Default|GetCityPiece) "/Game/Geometry/Meshes/City/SM_City_0.SM_City_0"))))
      (:1
        (if (Variables|Default|GetisSolarPowered)
          (Components|StaticMesh|SetStaticMesh (Variables|Default|GetCityPiece) "/Game/Geometry/Meshes/City/SM_City_1_Solar.SM_City_1_Solar")
          (else
            (Components|StaticMesh|SetStaticMesh (Variables|Default|GetCityPiece) "/Game/Geometry/Meshes/City/SM_City_1.SM_City_1"))))
      (:2
        (if (Variables|Default|GetisSolarPowered)
          (Components|StaticMesh|SetStaticMesh (Variables|Default|GetCityPiece) "/Game/Geometry/Meshes/City/SM_City_2_Solar.SM_City_2_Solar")
          (else
            (Components|StaticMesh|SetStaticMesh (Variables|Default|GetCityPiece) "/Game/Geometry/Meshes/City/SM_City_2.SM_City_2"))))
      (:3
        (if (Variables|Default|GetisSolarPowered)
          (Components|StaticMesh|SetStaticMesh (Variables|Default|GetCityPiece) "/Game/Geometry/Meshes/City/SM_City_3_Solar.SM_City_3_Solar")
          (else
            (Components|StaticMesh|SetStaticMesh (Variables|Default|GetCityPiece) "/Game/Geometry/Meshes/City/SM_City_3.SM_City_3")))))
    (CallFunction|RotateRandom)))

(fn RotateRandom
  (switch int (Math|Random|RandomIntegerinRange 1 4)
    (:1
      (Variables|Default|SetRotator "0, 0, 0"))
    (:2
      (Variables|Default|SetRotator "0.000000,90.000000,0.000000"))
    (:3
      (Variables|Default|SetRotator "0.000000,180.000000,0.000000"))
    (:4
      (Variables|Default|SetRotator "0.000000,270.000000,0.000000")))
  (Transformation|SetWorldRotation (Variables|Default|GetCityPiece) (Variables|Default|GetRotator) false false))

(fn UpgradeCity
  (if (not (or (== (Variables|Default|GetType) 3) (Variables|Default|GetisDisplayOnly)))
    (bind _result (Math|Integer|IncrementInt (Variables|Default|GetType))
      (:%20%20
        (switch int _result
          (:1
            (Components|StaticMesh|SetStaticMesh (Variables|Default|GetCityPiece) "/Game/Geometry/Meshes/City/SM_City_1.SM_City_1")
            (Rendering|Material|SetScalarParameterValueonMaterials (Variables|Default|GetCityPiece) "ONOFF" 2.0))
          (:2
            (Components|StaticMesh|SetStaticMesh (Variables|Default|GetCityPiece) "/Game/Geometry/Meshes/City/SM_City_2.SM_City_2")
            (Rendering|Material|SetScalarParameterValueonMaterials (Variables|Default|GetCityPiece) "ONOFF" 2.0))
          (:3
            (Components|StaticMesh|SetStaticMesh (Variables|Default|GetCityPiece) "/Game/Geometry/Meshes/City/SM_City_3.SM_City_3")
            (Rendering|Material|SetScalarParameterValueonMaterials (Variables|Default|GetCityPiece) "ONOFF" 2.0)))))))

(fn UpgradeCitySolar
  (if (not (Variables|Default|GetisDisplayOnly))
    (switch int (Variables|Default|GetType)
      (:1
        (Components|StaticMesh|SetStaticMesh (Variables|Default|GetCityPiece) "/Game/Geometry/Meshes/City/SM_City_1_Solar.SM_City_1_Solar")
        (Rendering|Material|SetScalarParameterValueonMaterials (Variables|Default|GetCityPiece) "ONOFF" 2.0))
      (:2
        (Components|StaticMesh|SetStaticMesh (Variables|Default|GetCityPiece) "/Game/Geometry/Meshes/City/SM_City_2_Solar.SM_City_2_Solar")
        (Rendering|Material|SetScalarParameterValueonMaterials (Variables|Default|GetCityPiece) "ONOFF" 2.0))
      (:3
        (Components|StaticMesh|SetStaticMesh (Variables|Default|GetCityPiece) "/Game/Geometry/Meshes/City/SM_City_3_Solar.SM_City_3_Solar")
        (Rendering|Material|SetScalarParameterValueonMaterials (Variables|Default|GetCityPiece) "ONOFF" 2.0)))))