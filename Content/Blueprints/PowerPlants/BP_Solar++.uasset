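; BP_Solar++ is an upgraded solar power plant that registers with the planet for its continent.
; Construction script scales build time and output from Planet's building data; Tick activates it after enough months, or when a timed deactivation expires.
; ChangeMesh switches active state, status sprite and Planet registration.
; Clicking toggles its UI_PowerPlant panel and selection highlight; intro state skips the build wait but registers it as BioFuel.
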(event OnClicked(clickable)
  (params (TouchedComponent :type Primitive%20Component%20Object%20Reference) (ButtonPressed :type Key%20Structure))
  (bind _struct (Variables|Default|GetStruct))
  (bind _widget (Variables|Default|GetWidget))
  (bind _staticmesh (Variables|Default|GetStaticMesh))
  (bind _returnvalue (UserInterface|GetWidget _widget))
  (bind (_asui_power_plant _bsuccess) (Utilities|Casting|CastToUI_PowerPlant _returnvalue))
  (if (not (Variables|Default|GetOnlyDisplay))
    (bind _outactors (Actor|GetAllActorsOfClass "/Game/Blueprints/PowerPlants/BP_PowerPlant.BP_PowerPlant_C"))
    (for _array_element _outactors
      (Rendering|Material|SetScalarParameterValueonMaterials (Variables|/Game/Blueprints/PowerPlants/BP_PowerPlant.BP_PowerPlant_C|GetStaticMesh _array_element) "Selector" 0.0))
    (Utilities|FlowControl|FlipFlop
      (:A
        (if _bsuccess
          (UserInterface|Viewport|AddtoViewport _asui_power_plant 0)
          (Default|SetType _asui_power_plant (.type _struct) (* (.energyproduction _struct) 2.0) (.usedcells _struct) (.carbonemissionpermwh _struct) (Variables|Default|Getorigin) (Variables|Default|GetTier))
          (Variables|/Game/UI/UI_PowerPlant.UI_PowerPlant_C|SetOwner _asui_power_plant self)
          (Variables|Default|Setactive_0 true)
          (Rendering|Material|SetScalarParameterValueonMaterials _staticmesh "Selector" 1.0)
          (else
            (Development|PrintString "CAST FAILED"))))
      (:B
        (Widget|RemovefromParent _asui_power_plant)
        (Variables|/Game/UI/UI_PowerPlant.UI_PowerPlant_C|SetOwner _asui_power_plant 0)
        (Variables|Default|Setactive_0 false)
        (Rendering|Material|SetScalarParameterValueonMaterials _staticmesh "Selector" 0.0)))))

(event EventBeginPlay
  (bind _planet (Variables|Default|GetPlanet))
  (if (not (Variables|Default|GetOnlyDisplay))
    (Variables|Default|Setinactive true)
    (bind _returnvalue (Class|MyActor|GetSelectedContinentID _planet))
    (Variables|Default|Setorigin (Utilities|Array|FindItem (Variables|/Game/PlanetGeneration.PlanetGeneration_C|GetContinentIDs _planet) _returnvalue))
    (if (Variables|/Game/PlanetGeneration.PlanetGeneration_C|GetIntroState (Variables|Default|GetPlanet))
      (Rendering|SetVisibility (Variables|Default|GetPaperSprite1) false false)
      (Default|AddorActivatePlant (Variables|Default|GetPlanet) "BioFuel" (Variables|Default|GetTier) (Variables|Default|Getorigin))
      (Variables|Default|Setinactive_0 false)
      (Variables|Default|Setinactive false))))

(event Collision|EventActorBeginOverlap
  (params (OtherActor :type Actor%20Object%20Reference))
  (|CallParentFunction OtherActor) ; This node is disabled and will not be called.\nDrag off pins to build functionality.
)

(event EventTick
  (params (DeltaSeconds :type Float%20%28single-precision%29))
  (if (>= (- (Variables|/Game/PlanetGeneration.PlanetGeneration_C|GetMonthsSurvived (Variables|Default|GetPlanet)) (Variables|Default|GetStartTime)) (Math|Float|Floor (Variables|Default|GetbuildTime))) :!label _label
    (if (and (>= (- (Variables|/Game/PlanetGeneration.PlanetGeneration_C|GetMonthsSurvived (Variables|Default|GetPlanet)) (Variables|Default|GetTimeofDeactivation)) (Variables|Default|GetDeactivationTime)) (Variables|Default|Getinactive_0))
      (Utilities|FlowControl|DoOnce false :!label _label_2
        (:Completed
          (CallFunction|ChangeMesh "Active")
          (goto _label_2 Reset)))
      (else
        (Utilities|FlowControl|DoOnce false
          (:Completed
            (Rendering|SetVisibility (Variables|Default|GetPaperSprite1) false false)
            (Default|AddorActivatePlant (Variables|Default|GetPlanet) "Solar" (Variables|Default|GetTier) (Variables|Default|Getorigin))
            (Variables|Default|Setinactive_0 false)
            (Variables|Default|Setinactive false)))))
    (else
      (Utilities|FlowControl|Delay 0.5)
      (goto _label))))

(fn ConstructionScript
  (bind _outactors (Actor|GetAllActorsOfClass "/Game/PlanetGeneration.PlanetGeneration_C"))
  (if (Utilities|IsValid (Utilities|Array|Get(acopy) _outactors))
    (bind _output_get (Variables|Default|SetPlanet (Utilities|Array|Get(acopy) _outactors))))
  (Variables|Default|SetbuildTime (* (.buildtime (.solar (Variables|/Game/PlanetGeneration.PlanetGeneration_C|GetBuildingStruct _output_get))) (.+time (Variables|/Game/PlanetGeneration.PlanetGeneration_C|GetBuildingStruct _output_get))))
  (Variables|Default|SetenergyProduction (* (.energyproduction (.solar (Variables|/Game/PlanetGeneration.PlanetGeneration_C|GetBuildingStruct _output_get))) (.+energy (Variables|/Game/PlanetGeneration.PlanetGeneration_C|GetBuildingStruct _output_get))))
  (Variables|Default|SetStartTime (Variables|/Game/PlanetGeneration.PlanetGeneration_C|GetMonthsSurvived _output_get))
  (if (Variables|Default|GetOnlyDisplay)
    (Rendering|SetVisibility (Variables|Default|GetPaperSprite1) false false)))

(fn ChangeMesh
  (params (NewStatus :type String) (DeactivationTime :type Integer))
  (bind _papersprite (Variables|Default|GetPaperSprite))
  (bind _origin (Variables|Default|Getorigin))
  (bind _planet (Variables|Default|GetPlanet))
  (bind _tier (Variables|Default|GetTier))
  (if (not (Variables|Default|GetOnlyDisplay))
    (switch string NewStatus
      (:Default
        (Components|StaticMesh|SetStaticMesh (Variables|Default|GetStaticMesh) "/Game/Geometry/Meshes/PowerPlants/SM_Solar++.SM_Solar++" :!label _label)
        (Rendering|SetVisibility _papersprite false false)
        (Variables|Default|Setinactive_0 false)
        (Default|AddorActivatePlant _planet "Solar" _tier _origin)
        (Variables|Default|Setinactive false))
      (:Active
        (goto _label))
      (:Inactive
        (Rendering|SetVisibility _papersprite true false)
        (Variables|Default|Setinactive_0 true)
        (Default|DiablePowerPlant _planet "Solar" _tier _origin)
        (Variables|Default|Setinactive true))
      (:DeactivateTime
        (Rendering|SetVisibility (Variables|Default|GetPaperSprite) true false)
        (Variables|Default|Setinactive_0 true)
        (Default|DiablePowerPlant (Variables|Default|GetPlanet) "Solar" (Variables|Default|GetTier) _origin)
        (Variables|Default|Setinactive true)
        (Variables|Default|SetTimeofDeactivation (Variables|/Game/PlanetGeneration.PlanetGeneration_C|GetMonthsSurvived (Variables|Default|GetPlanet)))
        (Variables|Default|SetDeactivationTime DeactivationTime)))))